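; BP_NumPad is a code-entry keypad that checks pressed digits against a target code and fires a dispatcher when they match.
; On BeginPlay it binds to the press dispatcher of every BP_NumPadButton actor in the level.
; Each press appends to the displayed input, which is compared once it reaches the target length.
; Success recolors the text and locks input; failure shows the failed color, then clears after a delay.
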(event Custom|NumPadButtonPressedDispatcher_Event_0
  (params (NumberPressed :type Integer))
  (bind _numpaddisplay (Variables|Default|GetNumPadDisplay))
  ;[1 1 1] Set up events to listen to key pad buttons
  (if (not (Variables|Default|GetCorrectCodeEntered)) ; If the correct code has been entered, lock the keypad input.
    (bind _output_get (Variables|Default|SetNumPadInput (Utilities|String|Append (Variables|Default|GetNumPadInput) (Utilities|String|ToString(Integer) NumberPressed))))
    (Rendering|Components|TextRender|SetText (Variables|Default|GetNumPadDisplay) (Utilities|Text|ToText(String) _output_get))
    (if (>= (Utilities|String|Len _output_get) (Utilities|String|Len (Variables|Default|GetTargetInputString)))
      (if (Utilities|Enum|Equal(Enum) (Variables|Default|GetNumPadInput) (Variables|Default|GetTargetInputString))
        ;[1 1 1] Successful code entered
        (Variables|Default|SetCorrectCodeEntered true)
        (Rendering|Components|TextRender|SetTextRenderColor (Variables|Default|GetNumPadDisplay) (Variables|Default|GetSuccessTextColor))
        (Default|CallCorrectCodeEnteredDispatcher)
        (else
          ;[1 1 1] Reset the number pad after a delay
          (Rendering|Components|TextRender|SetTextRenderColor (Variables|Default|GetNumPadDisplay) (Variables|Default|GetFailedTextColor))
          (Utilities|FlowControl|Delay 1.6)
          (bind _output_get_2 (Variables|Default|SetNumPadInput (Variables|Default|GetEmptyString)))
          (Rendering|Components|TextRender|SetText _numpaddisplay (Utilities|Text|ToText(String) _output_get_2))
          (Rendering|Components|TextRender|SetTextRenderColor _numpaddisplay (Variables|Default|GetDefaultTextColor)))))))

(event Custom|CorrectCodeEnteredDispatcher_Event
  ;[1 1 1] Set up events to listen to key pad buttons
)

(event EventBeginPlay
  ;[1 1 1] Set up events to listen to key pad buttons
  (EventDispatchers|BindEventtoCorrectCodeEnteredDispatcher (delegate Custom|CorrectCodeEnteredDispatcher_Event))
  (bind _outactors (Actor|GetAllActorsOfClass "/Game/NumPad/BP_NumPadButton_.BP_NumPadButton__C"))
  (for _array_element _outactors
    (EventDispatchers|AssignNumPadButtonPressedDispatcher _array_element (delegate Custom|NumPadButtonPressedDispatcher_Event_0))))

(fn ConstructionScript)