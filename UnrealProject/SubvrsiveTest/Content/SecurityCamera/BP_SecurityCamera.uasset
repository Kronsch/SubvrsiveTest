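; A security camera actor that changes its spotlight color to show how clearly it sees the player.
; On BeginPlay and every Tick, it rescales its detection sphere from an exposed radius and checks for player overlap.
; Inside the sphere, the dot product of camera forward and direction to the player selects red, yellow or green using two tolerances.
; Outside it, the light is green; each state also prints a debug string.
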(event EventTick
  (params (DeltaSeconds :type Float%20%28single-precision%29))
  (bind _returnvalue (Transformation|GetActorForwardVector))
  (bind _returnvalue_2 (Game|GetPlayerCharacter 0))
  (bind _returnvalue_3 (Transformation|GetActorLocation))
  (bind _spotlight (Variables|Default|GetSpotLight))
  (bind _returnvalue_4 (Math|Vector|Normalize _returnvalue))
  (bind _returnvalue_5 (Transformation|GetActorLocation _returnvalue_2))
  (bind _returnvalue_6 (- _returnvalue_5 _returnvalue_3))
  (bind _returnvalue_7 (Math|Vector|Normalize _returnvalue_6))
  (bind _returnvalue_8 (Math|Vector|DotProduct _returnvalue_7 _returnvalue_4))
  (Transformation|SetRelativeScale3D (Variables|Default|GetDetectionSphere) (Math|Conversions|ToVector(Float) (Variables|Default|GetDetectionSphereRadius))) ; Resize the detection sphere based on the exposed parameter.
  (if (Collision|IsOverlappingActor (Variables|Default|GetDetectionSphere) _returnvalue_2 :!class /Script/Engine.PrimitiveComponent) ; If we're not overlapping the detection sphere, default to green light.
    (if (> _returnvalue_8 (Variables|Default|GetDetectionAngleTolerance)) ; If the dot product is greater than Detection Angle Tolerance, player is in\nclear view of the security camera. Red light.
      (Rendering|Components|Light|SetLightColor _spotlight (Math|Conversions|ToLinearColor(Color) (Variables|Default|GetRedLightColor)) true)
      (Development|PrintString "RED")
      (elif (> _returnvalue_8 (Variables|Default|GetWarningAngleTolerance)) ; If the dot product is less than Detection Angle Tolerance, but\ngreater than Warning Angle Tolerance, player is just out of view.\nYellow light. False here means the player is clearly out of view.
        (Rendering|Components|Light|SetLightColor _spotlight (Math|Conversions|ToLinearColor(Color) (Variables|Default|GetYellowLightColor)) true)
        (Development|PrintString "YELLOW")
        (else
          (Rendering|Components|Light|SetLightColor _spotlight (Math|Conversions|ToLinearColor(Color) (Variables|Default|GetGreenLightColor)) true :!label _label)
          (Development|PrintString "GREEN"))))
    (else
      (goto _label))))

(event EventBeginPlay
  (bind _returnvalue (Transformation|GetActorForwardVector))
  (bind _returnvalue_2 (Game|GetPlayerCharacter 0))
  (bind _returnvalue_3 (Transformation|GetActorLocation))
  (bind _spotlight (Variables|Default|GetSpotLight))
  (bind _returnvalue_4 (Math|Vector|Normalize _returnvalue))
  (bind _returnvalue_5 (Transformation|GetActorLocation _returnvalue_2))
  (bind _returnvalue_6 (- _returnvalue_5 _returnvalue_3))
  (bind _returnvalue_7 (Math|Vector|Normalize _returnvalue_6))
  (bind _returnvalue_8 (Math|Vector|DotProduct _returnvalue_7 _returnvalue_4))
  (Transformation|SetRelativeScale3D (Variables|Default|GetDetectionSphere) (Math|Conversions|ToVector(Float) (Variables|Default|GetDetectionSphereRadius))) ; Resize the detection sphere based on the exposed parameter.
  (if (Collision|IsOverlappingActor (Variables|Default|GetDetectionSphere) _returnvalue_2 :!class /Script/Engine.PrimitiveComponent) ; If we're not overlapping the detection sphere, default to green light.
    (if (> _returnvalue_8 (Variables|Default|GetDetectionAngleTolerance)) ; If the dot product is greater than Detection Angle Tolerance, player is in\nclear view of the security camera. Red light.
      (Rendering|Components|Light|SetLightColor _spotlight (Math|Conversions|ToLinearColor(Color) (Variables|Default|GetRedLightColor)) true)
      (Development|PrintString "RED")
      (elif (> _returnvalue_8 (Variables|Default|GetWarningAngleTolerance)) ; If the dot product is less than Detection Angle Tolerance, but\ngreater than Warning Angle Tolerance, player is just out of view.\nYellow light. False here means the player is clearly out of view.
        (Rendering|Components|Light|SetLightColor _spotlight (Math|Conversions|ToLinearColor(Color) (Variables|Default|GetYellowLightColor)) true)
        (Development|PrintString "YELLOW")
        (else
          (Rendering|Components|Light|SetLightColor _spotlight (Math|Conversions|ToLinearColor(Color) (Variables|Default|GetGreenLightColor)) true :!label _label)
          (Development|PrintString "GREEN"))))
    (else
      (goto _label))))

(fn ConstructionScript)